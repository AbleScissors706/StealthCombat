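; BP_Lever is an interactable lever that plays a sound and triggers a linked actor when used.
; Interact calls SwitchLever, which sends InteractMessage to OutputVector through BPI_Interact on every pull.
; It also flips Activated and plays or reverses the PullLever timeline to rotate the Lever component.
; Without a valid target implementing that interface, only the sound plays and the lever stays put.
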(event Custom|SwitchLever
  (Audio|PlaySoundatLocation "/Engine/VREditor/Sounds/UI/Floating_UI_Close-001.Floating_UI_Close-001" (Transformation|GetActorLocation) "0, 0, 0" 1.0 1.0 0.0 "/Game/Audio/Grunts/SA_Sensor.SA_Sensor" 0 0 0)
  (bind _outputvector (Variables|Default|GetOutputVector)
    (:then
      (if (Utilities|DoesObjectImplementInterface _outputvector "/Game/Blueprints/BPI_Interact.BPI_Interact_C")
        (Class|BPIInteract|Interact(Message) _outputvector)
        (if (not (Variables|Default|GetActivated))
          (Variables|Default|SetActivated true)
          (bind _rotation (Timeline|PullLever Play)
            (:Update
              (Transformation|SetRelativeRotation (Variables|Default|GetLever) (Math|Rotator|Lerp(Rotator) "120.000000,0.000000,0.000000" "50.000000,0.000000,0.000000" _rotation) false false)))
          (else
            (Variables|Default|SetActivated false)
            (Timeline|PullLever Reverse)))))
    (:else)))

(event EventBeginPlay)

(event Collision|EventActorBeginOverlap
  (params (OtherActor :type Actor%20Object%20Reference)))

(event EventTick
  (params (DeltaSeconds :type Float%20%28single-precision%29)))

(event EventInteract
  (CallFunction|SwitchLever))

(fn ConstructionScript)