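; BP_Alarm is an alarm actor for a stealth game that raises all guards when triggered.
; StartAlarm spawns the alarm sound at the actor's location once, then AlertGuards sets HasSeenPlayer on each guard's AI blackboard and has the game mode switch music to escaping.
; StopAlarm is meant to fade out the sound, but its inverted AlarmActive check skips this while the alarm is active.
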(event Custom|StartAlarm
  ;[1 1 1] Start Alarm
  (if (not (Variables|Default|GetAlarmActive))
    (bind _returnvalue (Audio|SpawnSoundatLocation "/Game/Audio/Alarms/MS_Alarm.MS_Alarm" (Transformation|GetActorLocation) "0, 0, 0" 1.0 1.0 0.0 0 0))
    (Variables|Default|SetAlarmSound _returnvalue)
    (Variables|Default|SetAlarmActive true)
    (CallFunction|AlertGuards)))

(event Custom|StopAlarm
  ;[1 1 1] Stop Alarm
  (if (not (Variables|Default|GetAlarmActive))
    (Audio|Components|Audio|FadeOut (Variables|Default|GetAlarmSound) 1.0 0.0 "Linear" :!class /Script/Engine.AudioComponent)
    (Variables|Default|SetAlarmActive false)))

(event Custom|AlertGuards
  (bind _outactors (Actor|GetAllActorsOfClass "/Game/AI/BP_Guard.BP_Guard_C"))
  (for _array_element _outactors
    (bind _asbp_ai_guard (Utilities|Casting|CastToBP_AI_Guard (AI|GetAIController _array_element)))
    (AI|Components|Blackboard|SetValueasBool (AI|GetBlackboard _asbp_ai_guard) (Utilities|Name|MakeLiteralName "HasSeenPlayer") true))
  (bind _asgm_stealth_game_mode (Utilities|Casting|CastToGM_StealthGameMode (Game|GetGameMode)))
  (Default|SwitchMusictoEscaping _asgm_stealth_game_mode))

(event EventBeginPlay)

(event Collision|EventActorBeginOverlap
  (params (OtherActor :type Actor%20Object%20Reference)))

(event EventTick
  (params (DeltaSeconds :type Float%20%28single-precision%29)))

(fn ConstructionScript)