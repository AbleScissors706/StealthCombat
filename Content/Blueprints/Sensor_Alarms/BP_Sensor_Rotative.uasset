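; Rotating alarm sensor that detects the player after accumulated exposure in its detection zone.
; A timeline and FlipFlop sweep the head back and forth continuously.
; Overlap by a Player-tagged actor starts a looping timer that grows exposure and fills the player's detection meter.
; At the threshold it calls DetectPlayer, clears the timer and flags the meter as detected; nothing here handles leaving the zone.
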(event OnComponentBeginOverlap(TriggerDetectionZone)
  (params (OverlappedComponent :type Primitive%20Component%20Object%20Reference) (OtherActor :type Actor%20Object%20Reference) (OtherComp :type Primitive%20Component%20Object%20Reference) (OtherBodyIndex :type Integer) (bFromSweep :type Boolean) (SweepResult :type Hit%20Result%20Structure%20%28by%20ref%29))
  (if (Actor|ActorHasTag OtherActor "Player")
    (Variables|Default|SetPlayerInZone true)
    (bind _returnvalue (Utilities|Time|SetTimerbyEvent (delegate Custom|Count) 0.002 true))
    (Variables|Default|SetCountTimer _returnvalue)))

(event Custom|Count
  (Variables|Default|SetTimeUnderZone (+ (Variables|Default|GetTimeUnderZone) 0.005))
  (CallFunction|UpdateProgressBar)
  (if (>= (Variables|Default|GetTimeUnderZone) 3.0)
    (CallFunction|DetectPlayer (stale OnComponentBeginOverlap(TriggerDetectionZone) OtherActor))
    (Utilities|Time|ClearandInvalidateTimerbyHandle (Variables|Default|GetCountTimer))
    (Default|Detected (Variables|/Game/Blueprints/BP_Player.BP_Player_C|GetDetectionMeterWidget (Variables|Default|GetPlayerBP)))))

(event Custom|UpdateProgressBar
  ;[1 1 1] UpdateProgressBar
  (Progress|SetPercent (Variables|/Game/UI/WB_DetectionMeter.WB_DetectionMeter_C|GetProgressBar (Variables|/Game/Blueprints/BP_Player.BP_Player_C|GetDetectionMeterWidget (Variables|Default|GetPlayerBP))) (/ (Variables|Default|GetTimeUnderZone) 3.0)))

(event Collision|EventActorBeginOverlap
  (params (OtherActor :type Actor%20Object%20Reference))
  (|CallParentFunction OtherActor) ; This node is disabled and will not be called.\nDrag off pins to build functionality.
)

(event EventTick
  (params (DeltaSeconds :type Float%20%28single-precision%29))
  (|CallParentFunction DeltaSeconds) ; This node is disabled and will not be called.\nDrag off pins to build functionality.
)

(event EventBeginPlay
  (Utilities|FlowControl|Sequence
    (:then_0
      (bind _rotation (Timeline|Motion Play)
        (:Update
          (Transformation|SetRelativeRotation (Variables|Default|GetHead) (Math|Rotator|Lerp(Rotator) "0.000000,90.000000,0.000000" "0.000000,-90.000000,0.000000" _rotation) false false))
        (:Finished
          (Utilities|FlowControl|FlipFlop
            (:A
              (Timeline|Motion Reverse))
            (:B
              (Timeline|Motion Play))))))
    (:then_1
      (bind _asbp_player (Utilities|Casting|CastToBP_Player (Game|GetPlayerCharacter 0)))
      (Variables|Default|SetPlayerBP _asbp_player))))

(fn ConstructionScript
  (|CallParentFunction))