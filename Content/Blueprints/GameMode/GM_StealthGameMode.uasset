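; GM_StealthGameMode is the game mode for a stealth game, handling background music and the captured screen.
; BeginPlay spawns and fades in the main music track.
; SwitchMusicToEscaping fades that track out and spawns the louder escape track.
; Captured creates the WB_Captured widget, adds it to the viewport and plays its fade animation.
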(event Custom|Captured
  (bind _returnvalue (UserInterface|CreateWidget "/Game/UI/WB_Captured.WB_Captured_C"))
  (bind _output_get (Variables|Default|SetCapturedWidget _returnvalue))
  (UserInterface|Viewport|AddtoViewport _output_get 0)
  (Default|FadeAnimation (Variables|Default|GetCapturedWidget)))

(event Custom|SwitchMusicToEscaping
  (Audio|Components|Audio|FadeOut (Variables|Default|GetMusic) 0.3 0.0 "Linear" :!class /Script/Engine.AudioComponent)
  (bind _returnvalue (Audio|SpawnSound2D "/Game/Audio/Music/Escaping.Escaping" 0.5 1.0 0.0 0))
  (Variables|Default|SetEscapingMusic _returnvalue))

(event EventBeginPlay
  (bind _returnvalue (Audio|SpawnSound2D "/Game/Audio/Music/Music.Music" 0.3 1.0 0.0 0))
  (bind _output_get (Variables|Default|SetMusic _returnvalue))
  (Audio|Components|Audio|FadeIn _output_get 0.3 1.0 0.0 "Linear" :!class /Script/Engine.AudioComponent))

(event EventTick
  (params (DeltaSeconds :type Float%20%28single-precision%29)))

(fn ConstructionScript)