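; BP_AI_Guard is a guard AI controller that runs BT_Guard and raises the alarm when it spots the player.
; On a successful sight stimulus from a Player-tagged actor, AI perception sets the HasSeenPlayer blackboard key for the behavior tree.
; A HasSeenPlayer flag, never reset here, limits the reaction to the first sighting: a shout at the guard's location, then StartAlarm on BP_Alarm after a short delay.
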(event OnTargetPerceptionUpdated(AIPerception)
  (params (Actor :type Actor%20Object%20Reference) (Stimulus :type AI%20Stimulus%20Structure))
  (bind _returnvalue (Class|AIPerceptionSystem|GetSenseClassforStimulus Stimulus))
  (if (== _returnvalue "/Script/AIModule.AISense_Sight")
    (if (and (.bSuccessfullySensed (Utilities|Struct|BreakAIStimulus Stimulus)) (Actor|ActorHasTag Actor "Player"))
      (AI|Components|Blackboard|SetValueasBool (AI|GetBlackboard 0) (Utilities|Name|MakeLiteralName "HasSeenPlayer") true)
      (if (not (Variables|Default|GetHasSeenPlayer))
        (Variables|Default|SetHasSeenPlayer true)
        (Audio|PlaySoundatLocation "/Game/Audio/Grunts/MS_Shout.MS_Shout" (Transformation|GetActorLocation (Components|GetOwner (Variables|Default|GetAIPerception))) "0, 0, 0" 1.0 1.0 0.0 "/Game/Audio/Grunts/SA_Sensor.SA_Sensor" 0 0 0)
        (Utilities|FlowControl|Delay 0.2)
        (bind _returnvalue_2 (Actor|GetActorOfClass "/Game/Blueprints/Sensor_Alarms/BP_Alarm.BP_Alarm_C"))
        (Default|StartAlarm _returnvalue_2)))))

(event EventBeginPlay
  (AI|RunBehaviorTree "/Game/AI/BT_Guard.BT_Guard"))

(event EventTick
  (params (DeltaSeconds :type Float%20%28single-precision%29)))

(fn ConstructionScript)